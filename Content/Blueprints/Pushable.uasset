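; Pushable cube that slides along the X or Y axis in fixed steps when the first-person character pushes it.
; Four side triggers set a direction away from the player, and a timeline lerps the cube's relative location without sweep.
; On finishing, it steps again if the player still overlaps a trigger.
; Overlaps with Static components, except on FloorSwitch actors, stop the timeline without clearing IsMoving.
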(event `self.Cube.OnComponentHit`
  (params (HitComponent :type "PrimitiveComponent Object Reference") (OtherActor :type "Actor Object Reference") (OtherComp :type "PrimitiveComponent Object Reference") (NormalImpulse :type "Vector Structure") (Hit :type "HitResult Structure (by ref)")))

(event `self.CubeCollision.OnComponentBeginOverlap`
  (params (OverlappedComponent :type "PrimitiveComponent Object Reference") (OtherActor :type "Actor Object Reference") (OtherComp :type "PrimitiveComponent Object Reference") (OtherBodyIndex :type Integer) (bFromSweep :type Boolean) (SweepResult :type "HitResult Structure (by ref)"))
  (bind _returnvalue (`GameplayStatics.GetObjectClass` OtherActor))
  (bind _lastlocation (`self.LastLocation`))
  (`KismetSystemLibrary.PrintString` (`KismetSystemLibrary.GetClassDisplayName` _returnvalue) :!label _label)
  (if (== _returnvalue "/Game/Blueprints/FloorSwitch.FloorSwitch_C")
    _
    (elif (`|EnumEquality` (`SceneComponent.Mobility` OtherComp) "Static")
      (bind (_direction _newtrack_2) (`Timeline|Timeline_0` :!via `Stop` :!label _label_2)
        (:`Update`
          (`SceneComponent.K2_SetRelativeLocation` (`self.Cube`) (`KismetMathLibrary.VLerp` _lastlocation (+ _lastlocation (* (`self.NewLocation`) 100.0)) _newtrack_2) false false))
        (:`Finished`
          (set `self.isMoving` false)
          (for _array_element (`self.GetOverlappingComponents` (`self.FPCharacter`))
            (if (== _array_element (`self.NegX`))
              (set `self.NewLocation` (1.0 0.0 0.0) :!label _label_3)
              (set `self.isMoving` true :!label _label_4)
              (set `self.LastLocation` (`SceneComponent.RelativeLocation` (`self.Cube`)))
              (goto _label_2 :!via `PlayFromStart`)
              (elif (== _array_element (`self.PosX`))
                (set `self.NewLocation` (-1.0 0.0 0.0) :!label _label_5)
                (goto _label_4)
                (elif (== _array_element (`self.NegY`))
                  (set `self.NewLocation` (0.0 1.0 0.0) :!label _label_6)
                  (goto _label_4)
                  (elif (== _array_element (`self.PosY`))
                    (set `self.NewLocation` (0.0 -1.0 0.0) :!label _label_7)
                    (goto _label_4)))))))))))

(event `self.Cube.OnComponentBeginOverlap`
  (params (OverlappedComponent :type "PrimitiveComponent Object Reference") (OtherActor :type "Actor Object Reference") (OtherComp :type "PrimitiveComponent Object Reference") (OtherBodyIndex :type Integer) (bFromSweep :type Boolean) (SweepResult :type "HitResult Structure (by ref)"))
  (goto _label))

(event `self.NegX.OnComponentBeginOverlap`
  (params (OverlappedComponent :type "PrimitiveComponent Object Reference") (OtherActor :type "Actor Object Reference") (OtherComp :type "PrimitiveComponent Object Reference") (OtherBodyIndex :type Integer) (bFromSweep :type Boolean) (SweepResult :type "HitResult Structure (by ref)"))
  (if (`self.isMoving`)
    _
    (elif (== (`GameplayStatics.GetObjectClass` OtherActor) "/Game/FirstPersonBP/Blueprints/FirstPersonCharacter.FirstPersonCharacter_C")
      (bind _asfirst_person_character (cast `/Game/FirstPersonBP/Blueprints/FirstPersonCharacter` OtherActor))
      (set `self.FPCharacter` _asfirst_person_character)
      (goto _label_3))))

(event `self.PosX.OnComponentBeginOverlap`
  (params (OverlappedComponent :type "PrimitiveComponent Object Reference") (OtherActor :type "Actor Object Reference") (OtherComp :type "PrimitiveComponent Object Reference") (OtherBodyIndex :type Integer) (bFromSweep :type Boolean) (SweepResult :type "HitResult Structure (by ref)"))
  (if (`self.isMoving`)
    _
    (elif (== (`GameplayStatics.GetObjectClass` OtherActor) "/Game/FirstPersonBP/Blueprints/FirstPersonCharacter.FirstPersonCharacter_C")
      (bind _asfirst_person_character (cast `/Game/FirstPersonBP/Blueprints/FirstPersonCharacter` OtherActor))
      (set `self.FPCharacter` _asfirst_person_character)
      (goto _label_5))))

(event `self.NegY.OnComponentBeginOverlap`
  (params (OverlappedComponent :type "PrimitiveComponent Object Reference") (OtherActor :type "Actor Object Reference") (OtherComp :type "PrimitiveComponent Object Reference") (OtherBodyIndex :type Integer) (bFromSweep :type Boolean) (SweepResult :type "HitResult Structure (by ref)"))
  (if (`self.isMoving`)
    _
    (elif (== (`GameplayStatics.GetObjectClass` OtherActor) "/Game/FirstPersonBP/Blueprints/FirstPersonCharacter.FirstPersonCharacter_C")
      (bind _asfirst_person_character (cast `/Game/FirstPersonBP/Blueprints/FirstPersonCharacter` OtherActor))
      (set `self.FPCharacter` _asfirst_person_character)
      (goto _label_6))))

(event `self.PosY.OnComponentBeginOverlap`
  (params (OverlappedComponent :type "PrimitiveComponent Object Reference") (OtherActor :type "Actor Object Reference") (OtherComp :type "PrimitiveComponent Object Reference") (OtherBodyIndex :type Integer) (bFromSweep :type Boolean) (SweepResult :type "HitResult Structure (by ref)"))
  (if (`self.isMoving`)
    _
    (elif (== (`GameplayStatics.GetObjectClass` OtherActor) "/Game/FirstPersonBP/Blueprints/FirstPersonCharacter.FirstPersonCharacter_C")
      (bind _asfirst_person_character (cast `/Game/FirstPersonBP/Blueprints/FirstPersonCharacter` OtherActor))
      (set `self.FPCharacter` _asfirst_person_character)
      (goto _label_7))))

(fn `UserConstructionScript`)