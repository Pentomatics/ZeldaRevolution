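; BossLeftHand is the left hand of a boss, which moves on a loop and shatters when hit by an arrow.
; A looping timeline adds a relative offset to the hand on every update, without sweeping.
; When an Arrow overlaps the capsule, it notifies its parent actor through the IGodhan interface, spawns DestructibleLeftHand at the hand's transform, destroys itself and plays a rock-shatter sound.
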(event `self.ReceiveBeginPlay`
  (bind (_direction _newtrack_1) (`Timeline|HandMvement` :!label _label)
    (:`Update`
      (`SceneComponent.K2_AddRelativeLocation` (`self.LeftHand`) _newtrack_1 false false))
    (:`Finished`
      (if true
        (goto _label :!via `PlayFromStart`)))))

(event `self.Capsule.OnComponentBeginOverlap`
  (params (OverlappedComponent :type "PrimitiveComponent Object Reference") (OtherActor :type "Actor Object Reference") (OtherComp :type "PrimitiveComponent Object Reference") (OtherBodyIndex :type Integer) (bFromSweep :type Boolean) (SweepResult :type "HitResult Structure (by ref)"))
  (bind _returnvalue (`self.GetParentActor` self))
  (if (== (`GameplayStatics.GetObjectClass` OtherActor) "/Game/Blueprints/Arrow.Arrow_C")
    (if (`KismetSystemLibrary.DoesImplementInterface` _returnvalue "/Game/Blueprints/IGodhan.IGodhan_C")
      (message `/Game/Blueprints/IGodhan.ActorDefeated` _returnvalue self))
    (`|SpawnActorFromClass` "/Game/Blueprints/DestructibleLeftHand.DestructibleLeftHand_C" (`SceneComponent.K2_GetComponentToWorld` (`self.LeftHand`)) "Undefined" "OverrideRootScale")
    (`self.K2_DestroyActor`)
    (`GameplayStatics.PlaySound2D` "/Game/Sounds/WW_Rock_Shatter.WW_Rock_Shatter")))

(fn `UserConstructionScript`)