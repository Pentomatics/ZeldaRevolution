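; Godhan boss actor that drifts along a looping path and tracks the defeat of its left and right hand child actors.
; On BeginPlay it caches the first FirstPersonCharacter and, if found, starts the CircleMovement timeline, which adds its vector track as a local root offset each update and restarts when finished.
; ActorDefeated flags each hand, but the both-defeated branch is empty.
; RotateStatue and MoveStatue run on Tick but are empty stubs.
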(event `self.ReceiveBeginPlay`
  (bind _outactors (`GameplayStatics.GetAllActorsOfClass` "/Game/FirstPersonBP/Blueprints/FirstPersonCharacter.FirstPersonCharacter_C"))
  (if (> (`KismetArrayLibrary.Array_Length` _outactors) 0)
    (set `self.Ref 2 FPCharacter` (`|GetArrayItem` _outactors))
    (bind (_direction _cyrclevector) (`Timeline|CircleMovement` :!label _label)
      (:`Update`
        (`SceneComponent.K2_AddLocalTransform` (`self.DefaultSceneRoot`) (`KismetMathLibrary.MakeTransform` _cyrclevector) false false))
      (:`Finished`
        (if true
          (goto _label :!via `PlayFromStart`))))))

(event `self.ReceiveTick`
  (params (DeltaSeconds :type "Float (single-precision)"))
  (`self.RotateStatue` DeltaSeconds)
  (`self.MoveStatue` DeltaSeconds))

(event `/Game/Blueprints/IGodhan.ActorDefeated`
  (params (DefeatedActor :type "Actor Object Reference"))
  (if (== DefeatedActor (`ChildActorComponent.ChildActor` (`self.BossLeftHand`)))
    (bind _output_get (set `self.isLeftHandDefeated` true))
    (if (and _output_get (stale _output_get_2)) :!label _label_2
      _)
    (elif (== DefeatedActor (`ChildActorComponent.ChildActor` (`self.BossRightHand`)))
      (bind _output_get_2 (set `self.isRightHandDefeated` true))
      (goto _label_2))))

(fn `MoveStatue`
  (params (DeltaSeconds :type "Float (double-precision)")))

(fn `RotateStatue`
  (params (DeltaSeconds :type "Float (double-precision)")))

(fn `UserConstructionScript`)