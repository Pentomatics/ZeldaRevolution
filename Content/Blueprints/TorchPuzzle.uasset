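; Torch puzzle actor that unlocks a temple door, held as a child actor, when every linked torch switch is lit.
; On the OnActorActivated event it checks each switch's OnFire state, then calls UnlockDoor and plays an item-get sound if all are burning.
; The construction script runs the same check to set the door's Unlocked flag from the torches' initial states.
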(event `/Game/Blueprints/ISolvable.OnActorActivated`
  (params (Actor :type "Actor Object Reference"))
  (set `self.shouldOpenDoor` true)
  (for _array_element (`self.torchSwitches`)
    (if (not (`/Game/Blueprints/TorchSwitch.onFire` _array_element))
      (set `self.shouldOpenDoor` false)))
  (bind _astemple_door (cast `/Game/Blueprints/TempleDoor` (`ChildActorComponent.ChildActor` (`self.TempleDoor`))))
  (if (`self.shouldOpenDoor`)
    (`/Game/Blueprints/TempleDoor.UnlockDoor` _astemple_door)
    (`GameplayStatics.PlaySound2D` "/Game/Sounds/WW_Get_Item.WW_Get_Item")))

(fn `UserConstructionScript`
  (set `self.shouldOpenDoor` true)
  (for _array_element (`self.torchSwitches`)
    (if (not (`/Game/Blueprints/TorchSwitch.onFire` _array_element))
      (set `self.shouldOpenDoor` false)))
  (bind _astemple_door (cast `/Game/Blueprints/TempleDoor` (`ChildActorComponent.ChildActor` (`self.TempleDoor`))))
  (set `/Game/Blueprints/TempleDoor.unlocked` (`self.shouldOpenDoor`) _astemple_door))