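; Statue actor that keeps turning toward the first-person camera and creeps forward while it is behind the player's view.
; BeginPlay enables Tick when an actor search finds a match; Tick then runs RotateStatue and MoveStatue.
; Rotation corrects pitch and yaw in proportion to the camera's relative angle, with roll locked to zero.
; Movement runs along local X only while the statue's yaw relative to the camera exceeds 90 degrees.
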(event `self.ReceiveBeginPlay`
  (bind _outactors (`GameplayStatics.GetAllActorsOfClass` null))
  (if (> (`KismetArrayLibrary.Array_Length` _outactors) 0)
    (set `self.Ref2FPCharacter` null)
    (`self.SetActorTickEnabled` true)))

(event `self.ReceiveTick`
  (params (DeltaSeconds :type "Float (single-precision)"))
  (`self.RotateStatue` DeltaSeconds)
  (`self.MoveStatue` DeltaSeconds))

(fn `MoveStatue`
  (params (DeltaSeconds :type "Float (double-precision)"))
  (bind (_returnvalue_roll _returnvalue_pitch _returnvalue_yaw) (`KismetMathLibrary.BreakRotator` (`KismetMathLibrary.MakeRotFromX` (.location (`KismetMathLibrary.ComposeTransforms` (`SceneComponent.K2_GetComponentToWorld` (`self.DefaultSceneRoot`)) (`KismetMathLibrary.InvertTransform` (`SceneComponent.K2_GetComponentToWorld` (`self.FirstPersonCamera`))))))))
  (if (> (`KismetMathLibrary.Abs` _returnvalue_yaw) 90.0)
    (`SceneComponent.K2_AddLocalOffset` (`self.DefaultSceneRoot`) (`KismetMathLibrary.MakeVector` (* DeltaSeconds (`self.MovementSpeed`) 100.0)) false false)))

(fn `RotateStatue`
  (params (DeltaSeconds :type "Float (double-precision)"))
  (bind _lookingspeed (`self.lookingSpeed`))
  (bind (_returnvalue_roll _returnvalue_pitch _returnvalue_yaw) (`KismetMathLibrary.BreakRotator` (`SceneComponent.K2_GetComponentRotation` (`self.DefaultSceneRoot`))))
  (bind (_returnvalue_roll_2 _returnvalue_pitch_2 _returnvalue_yaw_2) (`KismetMathLibrary.BreakRotator` (`KismetMathLibrary.MakeRotFromX` (.location (`KismetMathLibrary.ComposeTransforms` (`SceneComponent.K2_GetComponentToWorld` (`self.FirstPersonCamera`)) (`KismetMathLibrary.InvertTransform` (`SceneComponent.K2_GetComponentToWorld` (`self.DefaultSceneRoot`))))))))
  ;[1 1 1] Fix: FacingActor soll sich niemals rollen!
  (`SceneComponent.K2_SetWorldRotation` (`self.DefaultSceneRoot`) (`KismetMathLibrary.MakeRotator` 0.0 (+ (* DeltaSeconds _returnvalue_pitch_2 _lookingspeed) _returnvalue_pitch) (+ _returnvalue_yaw (* _lookingspeed DeltaSeconds _returnvalue_yaw_2))) false false))

(fn `UserConstructionScript`)