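; Grenade actor that explodes when it hits an actor whose display name is "testCube".
; The Hit event disables gravity and enables physics on the struck component, then applies a vertical impulse scaled by ExplosionStrength.
; It spawns an explosion particle at the grenade mesh's location and destroys itself.
; Activate is empty, and a disconnected branch that sets HasGrenade and destroys the actor never runs.
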(event `self.ReceiveHit`
  (params (MyComp :type "PrimitiveComponent Object Reference") (Other :type "Actor Object Reference") (OtherComp :type "PrimitiveComponent Object Reference") (bSelfMoved :type Boolean) (HitLocation :type "Vector Structure") (HitNormal :type "Vector Structure") (NormalImpulse :type "Vector Structure") (Hit :type "HitResult Structure (by ref)"))
  (if (`KismetStringLibrary.EqualEqual_StrStr` (`KismetSystemLibrary.GetDisplayName` Other) "testCube")
    (`PrimitiveComponent.SetEnableGravity` OtherComp false)
    (`PrimitiveComponent.SetSimulatePhysics` OtherComp true)
    (`PrimitiveComponent.AddImpulse` OtherComp (`KismetMathLibrary.MakeVector` 0.0 0.0 (`self.ExplosionStrength`)) "None" false)
    (`GameplayStatics.SpawnEmitterAtLocation` "/Game/StarterContent/Particles/P_Explosion.P_Explosion" (`SceneComponent.K2_GetComponentLocation` (`self.Granade_low`)))
    (`self.K2_DestroyActor`)))

(event `Activate`)

(fn `UserConstructionScript`)