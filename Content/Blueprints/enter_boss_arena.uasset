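; Trigger actor that marks the player's entry into the boss arena, destroying the bridge and switching the music.
; Its box overlap checks for the FirstPersonCharacter class and runs the sequence only once.
; It destroys the referenced Bridge, briefly fades out the first-half music, silences the level's main music instantly and activates the second-half track.
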(event `self.Box.OnComponentBeginOverlap`
  (params (OverlappedComponent :type "PrimitiveComponent Object Reference") (OtherActor :type "Actor Object Reference") (OtherComp :type "PrimitiveComponent Object Reference") (OtherBodyIndex :type Integer) (bFromSweep :type Boolean) (SweepResult :type "HitResult Structure (by ref)"))
  ;[1 1 1] if player enters
  (if (== (`GameplayStatics.GetObjectClass` OtherActor) "/Game/FirstPersonBP/Blueprints/FirstPersonCharacter.FirstPersonCharacter_C")
    (`/Engine/EditorBlueprintResources/StandardMacros.DoOnce` false
      (:`Completed`
        ;[1 1 1] destroy bridge
        (`self.K2_DestroyActor` (`self.bridge`))
        ;[1 1 1] change music
        (`AudioComponent.AdjustVolume` (`AmbientSound.AudioComponent` (`self.first half music`)) 0.5 0.0)
        (`AudioComponent.AdjustVolume` (`AmbientSound.AudioComponent` (`self.level main music`)) 0.0 0.0)
        (`ActorComponent.Activate` (`AmbientSound.AudioComponent` (`self.second half music`)) false)))))

(fn `UserConstructionScript`)