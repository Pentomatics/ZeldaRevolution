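; GodhanHead is a boss head that bobs or drifts on a looping timeline and turns proportionally toward the player camera, with limited pitch and no roll.
; It stays immortal until ActorDefeated has reported both child-actor hands.
; Arrow overlaps then flag each eye.
; With both eyes hit, it spawns a destructible head, destroys itself, plays a victory sound, switches to boss-clear music and fades the camera out.
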(event `self.ReceiveTick`
  (params (DeltaSeconds :type "Float (single-precision)"))
  (if (not (`self.isHeadDefeated`))
    (`self.RotateStatue` DeltaSeconds)))

(event `self.CollisionLeftEye.OnComponentBeginOverlap`
  (params (OverlappedComponent :type "PrimitiveComponent Object Reference") (OtherActor :type "Actor Object Reference") (OtherComp :type "PrimitiveComponent Object Reference") (OtherBodyIndex :type Integer) (bFromSweep :type Boolean) (SweepResult :type "HitResult Structure (by ref)"))
  (if (`self.immortal`)
    _
    (elif (== (`GameplayStatics.GetObjectClass` OtherActor) "/Game/Blueprints/Arrow.Arrow_C")
      ;[1 1 1] left eye hit event
      (set `self.hitLeftEye` true)
      (`|ExecutionSequence` :!label _label
        (:`then_0`
          (if (and (`self.hitLeftEye`) (`self.hitRightEye`))
            (`|SpawnActorFromClass` "/Game/Blueprints/DestructibleHead.DestructibleHead_C" (`SceneComponent.K2_GetComponentToWorld` (`self.Head`)) "Undefined" "OverrideRootScale")
            (`self.K2_DestroyActor`)
            ;[1 1 1] you win!
            (`GameplayStatics.PlaySound2D` "/Game/Sounds/Gohdan/Shiren_0_aw_00000006.Shiren_0_aw_00000006" 0.8)
            (`AudioComponent.AdjustVolume` (`AmbientSound.AudioComponent` (`self.second half music`)) 0.5 0.0)
            (`ActorComponent.Activate` (`AmbientSound.AudioComponent` (`self.boss clear music`)) false)
            (`PlayerCameraManager.StartCameraFade` :`self` (`GameplayStatics.GetPlayerCameraManager` 0) :`ToAlpha` 1.0 :`Duration` 5.0 :`bHoldWhenFinished` true)))
        (:`then_1`
          ;[1 1 1] eye hit effects
          (`GameplayStatics.PlaySound2D` "/Game/Sounds/WW_Rock_Shatter_Impact.WW_Rock_Shatter_Impact"))))))

(event `self.CollisiontRightEye.OnComponentBeginOverlap`
  (params (OverlappedComponent :type "PrimitiveComponent Object Reference") (OtherActor :type "Actor Object Reference") (OtherComp :type "PrimitiveComponent Object Reference") (OtherBodyIndex :type Integer) (bFromSweep :type Boolean) (SweepResult :type "HitResult Structure (by ref)"))
  (if (`self.immortal`)
    _
    (elif (== (`GameplayStatics.GetObjectClass` OtherActor) "/Game/Blueprints/Arrow.Arrow_C")
      ;[1 1 1] right eye hit event
      (set `self.hitRightEye` true)
      (goto _label))))

(event `self.ReceiveBeginPlay`
  (bind _outactors (`GameplayStatics.GetAllActorsOfClass` "/Game/FirstPersonBP/Blueprints/FirstPersonCharacter.FirstPersonCharacter_C"))
  (if (> (`KismetArrayLibrary.Array_Length` _outactors) 0)
    (set `self.Ref2FPCharacter` (`|GetArrayItem` _outactors))
    (bind (_direction _cyrclevector) (`Timeline|Timeline_0` :!label _label_2)
      (:`Update`
        (`SceneComponent.K2_AddLocalTransform` (`self.DefaultSceneRoot`) (`KismetMathLibrary.MakeTransform` _cyrclevector) false false))
      (:`Finished`
        (if (not (`self.isHeadDefeated`))
          (goto _label_2 :!via `PlayFromStart`))))))

(event `/Game/Blueprints/IGodhan.ActorDefeated`
  (params (DefeatedActor :type "Actor Object Reference"))
  (if (== DefeatedActor (`ChildActorComponent.ChildActor` (`self.BossRightHand`)))
    (bind _output_get (set `self.isLeftHandDefeated` true))
    (if (and _output_get (stale _output_get_2)) :!label _label_3
      (set `self.immortal` false))
    (elif (== DefeatedActor (`ChildActorComponent.ChildActor` (`self.BossLeftHand`)))
      (bind _output_get_2 (set `self.isRightHandDefeated` true))
      (goto _label_3))))

(fn `RotateStatue`
  (params (DeltaSeconds :type "Float (double-precision)"))
  (bind _lookingspeed (`self.LookingSpeed`))
  (bind (_returnvalue_roll _returnvalue_pitch _returnvalue_yaw) (`KismetMathLibrary.BreakRotator` (`SceneComponent.K2_GetComponentRotation` (`self.Head`))))
  (bind (_returnvalue_roll_2 _returnvalue_pitch_2 _returnvalue_yaw_2) (`KismetMathLibrary.BreakRotator` (`KismetMathLibrary.MakeRotFromX` (.location (`KismetMathLibrary.ComposeTransforms` (`SceneComponent.K2_GetComponentToWorld` (`/Game/FirstPersonBP/Blueprints/FirstPersonCharacter.FirstPersonCamera` (`self.Ref2FPCharacter`))) (`KismetMathLibrary.InvertTransform` (`SceneComponent.K2_GetComponentToWorld` (`self.Head`))))))))
  (bind _returnvalue (+ (* DeltaSeconds _returnvalue_pitch_2 _lookingspeed) _returnvalue_pitch))
  (bind _returnvalue_2 (+ _returnvalue_yaw (* _lookingspeed _returnvalue_yaw_2 DeltaSeconds)))
  (if (and (>= _returnvalue -40.0) (<= _returnvalue 40.0))
    ;[1 1 1] Fix: FacingActor soll sich niemals rollen!
    (`SceneComponent.K2_SetWorldRotation` (`self.Head`) (`KismetMathLibrary.MakeRotator` 0.0 _returnvalue _returnvalue_2) false false)
    (else
      ;[1 1 1] Fix: FacingActor soll sich niemals rollen!
      (`SceneComponent.K2_SetWorldRotation` (`self.Head`) (`KismetMathLibrary.MakeRotator` 0.0 _returnvalue_pitch _returnvalue_2) false false))))

(fn `UserConstructionScript`)