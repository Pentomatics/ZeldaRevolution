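; SailBoat is a boat actor that carries out a scripted sail to a destination, then opens the Dungeon level.
; Release enables physics on the boat and arms the trigger, so a FirstPersonCharacter overlap starts sailing, which can also start on BeginPlay via SailOnStartGame.
; Sailing disables physics and move input while a Timeline lerps the boat between captured world locations, applied as relative location, restoring input on finish.
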(event `/Game/Blueprints/IReleaseable.release`
  (set `self.is boat released` true)
  (`PrimitiveComponent.SetSimulatePhysics` (`self.SailingBoat`) true))

(event `self.ReceiveBeginPlay`
  (if (`self.sail on start game`)
    (`self.start sail timeline`)))

(event `self.StartSailingTrigger.OnComponentBeginOverlap`
  (params (OverlappedComponent :type "PrimitiveComponent Object Reference") (OtherActor :type "Actor Object Reference") (OtherComp :type "PrimitiveComponent Object Reference") (OtherBodyIndex :type Integer) (bFromSweep :type Boolean) (SweepResult :type "HitResult Structure (by ref)"))
  (if (`self.is boat released`)
    (if (== (`GameplayStatics.GetObjectClass` OtherActor) "/Game/FirstPersonBP/Blueprints/FirstPersonCharacter.FirstPersonCharacter_C")
      (`self.start sail timeline`))))

(event `start sail timeline`
  ;[1 1 1] Restrict movement while sailing
  (bind _outactors (`GameplayStatics.GetAllActorsOfClass` "/Game/FirstPersonBP/Blueprints/FirstPersonCharacter.FirstPersonCharacter_C"))
  (bind _returnvalue (`GameplayStatics.GetPlayerController` (`|GetArrayItem` _outactors)))
  (`Controller.SetIgnoreMoveInput` _returnvalue true)
  (`PrimitiveComponent.SetSimulatePhysics` (`self.SailingBoat`) false)
  (set `self.start location` (`SceneComponent.K2_GetComponentLocation` (`self.SailingBoat`)))
  (set `self.targetLocation` (`SceneComponent.K2_GetComponentLocation` (`self.SailingTargetDestination`)))
  (bind (_direction _newtrack_1) (`Timeline|Timeline_0`)
    (:`Update`
      ;[1 1 1] Aktualisierung der Position
      (`SceneComponent.K2_SetRelativeLocation` (`self.SailingBoat`) (`KismetMathLibrary.VLerp` (`self.start location`) (`self.targetLocation`) _newtrack_1) false false))
    (:`Finished`
      (`Controller.ResetIgnoreMoveInput` _returnvalue)
      (`GameplayStatics.OpenLevel` "Dungeon"))))

(fn `UserConstructionScript`)