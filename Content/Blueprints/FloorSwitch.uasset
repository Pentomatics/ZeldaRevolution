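; FloorSwitch is a floor switch that registers as pressed while a PushableBlock sits in its Trigger.
; Begin and end overlap events set and clear the ButtonPressed flag and print a debug string.
; Both events require an exact PushableBlock class and a StaticMeshComponent as the overlapping component.
; It keeps no overlap count, so any qualifying exit clears the flag.
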(event `self.Trigger.OnComponentBeginOverlap`
  (params (OverlappedComponent :type "PrimitiveComponent Object Reference") (OtherActor :type "Actor Object Reference") (OtherComp :type "PrimitiveComponent Object Reference") (OtherBodyIndex :type Integer) (bFromSweep :type Boolean) (SweepResult :type "HitResult Structure (by ref)"))
  (if (and (== (`GameplayStatics.GetObjectClass` OtherActor) "/Game/Blueprints/PushableBlock.PushableBlock_C") (== (`GameplayStatics.GetObjectClass` OtherComp) "/Script/Engine.StaticMeshComponent"))
    (set `self.ButtonPressed` true)
    (`KismetSystemLibrary.PrintString` "pressed")))

(event `self.Trigger.OnComponentEndOverlap`
  (params (OverlappedComponent :type "PrimitiveComponent Object Reference") (OtherActor :type "Actor Object Reference") (OtherComp :type "PrimitiveComponent Object Reference") (OtherBodyIndex :type Integer))
  (if (and (== (`GameplayStatics.GetObjectClass` OtherActor) "/Game/Blueprints/PushableBlock.PushableBlock_C") (== (`GameplayStatics.GetObjectClass` OtherComp) "/Script/Engine.StaticMeshComponent"))
    (set `self.ButtonPressed` false)
    (`KismetSystemLibrary.PrintString` "not....")))

(fn `UserConstructionScript`)