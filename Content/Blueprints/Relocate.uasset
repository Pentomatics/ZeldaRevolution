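; Relocate is a trigger-volume actor that moves the first-person player to a referenced Spawn actor's location.
; When its Box begins overlapping an actor whose class is exactly FirstPersonCharacter and Spawn is valid, it stops that character's movement immediately.
; It then sets the character's location to Spawn's position without sweep or physics teleport, leaving rotation untouched.
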(event `self.Box.OnComponentBeginOverlap`
  (params (OverlappedComponent :type "PrimitiveComponent Object Reference") (OtherActor :type "Actor Object Reference") (OtherComp :type "PrimitiveComponent Object Reference") (OtherBodyIndex :type Integer) (bFromSweep :type Boolean) (SweepResult :type "HitResult Structure (by ref)"))
  (bind _spawn (`self.Spawn`))
  (if (== (`GameplayStatics.GetObjectClass` OtherActor) "/Game/FirstPersonBP/Blueprints/FirstPersonCharacter.FirstPersonCharacter_C")
    (if (`KismetSystemLibrary.IsValid` _spawn)
      (bind _asfirst_person_character (cast `/Game/FirstPersonBP/Blueprints/FirstPersonCharacter` OtherActor))
      (`MovementComponent.StopMovementImmediately` (`Pawn.GetMovementComponent` _asfirst_person_character))
      (`self.K2_SetActorLocation` OtherActor (`self.K2_GetActorLocation` _spawn) false false))))

(fn `UserConstructionScript`)