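; Buildable raft that the player assembles from planks, then rides to the Pirate_ship level.
; Construction script caches original materials and shows unbuilt meshes in green.
; Each Activate spends one of the character's planks to restore the next mesh's material and blocking collision until built.
; Boarding the built raft, or an optional start flag, locks move input and timeline-lerps it toward the ChangeLevelTrigger, whose overlap opens the level.
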(event `self.ReceiveBeginPlay`
  (if (`self.sail on start game`)
    (`self.start sail timeline`)))

(event `self.SailingTrigger.OnComponentBeginOverlap`
  (params (OverlappedComponent :type "PrimitiveComponent Object Reference") (OtherActor :type "Actor Object Reference") (OtherComp :type "PrimitiveComponent Object Reference") (OtherBodyIndex :type Integer) (bFromSweep :type Boolean) (SweepResult :type "HitResult Structure (by ref)"))
  (if (and (== (`GameplayStatics.GetObjectClass` OtherActor) "/Game/FirstPersonBP/Blueprints/FirstPersonCharacter.FirstPersonCharacter_C") (`self.is build`))
    (`self.start sail timeline`)))

(event `/Game/FirstPersonBP/ITraceable.Activate`
  (params (Character :type "/Game/FirstPersonBP/Blueprints/FirstPersonCharacter Object Reference") (Component :type "ActorComponent Object Reference"))
  (if (not (`self.is build`))
    (`self.build` Character)))

(event `start sail timeline`
  ;[1 1 1] Restrict movement while sailing
  (bind _outactors (`GameplayStatics.GetAllActorsOfClass` "/Game/FirstPersonBP/Blueprints/FirstPersonCharacter.FirstPersonCharacter_C"))
  (bind _returnvalue (`GameplayStatics.GetPlayerController` (`|GetArrayItem` _outactors)))
  (`Controller.SetIgnoreMoveInput` _returnvalue true)
  (set `self.start location` (`SceneComponent.RelativeLocation` (`self.Raft`)))
  (bind (_direction _newtrack_1) (`Timeline|sailing`)
    (:`Update`
      ;[1 1 1] Aktualisierung der Position
      (`SceneComponent.K2_SetRelativeLocation` (`self.Raft`) (`KismetMathLibrary.VLerp` (`self.start location`) (`SceneComponent.RelativeLocation` (`self.ChangeLevelTrigger`)) _newtrack_1) false false))
    (:`Finished`
      (`Controller.ResetIgnoreMoveInput` _returnvalue))))

(event `self.ChangeLevelTrigger.OnComponentBeginOverlap`
  (params (OverlappedComponent :type "PrimitiveComponent Object Reference") (OtherActor :type "Actor Object Reference") (OtherComp :type "PrimitiveComponent Object Reference") (OtherBodyIndex :type Integer) (bFromSweep :type Boolean) (SweepResult :type "HitResult Structure (by ref)"))
  (if (== (`GameplayStatics.GetObjectClass` OtherActor) "/Game/FirstPersonBP/Blueprints/FirstPersonCharacter.FirstPersonCharacter_C")
    (`GameplayStatics.OpenLevel` "Pirate_ship")))

(fn `build`
  (params (character :type "/Game/FirstPersonBP/Blueprints/FirstPersonCharacter Object Reference"))
  (bind _build_state (`self.Build State`))
  (bind _output (`|GetArrayItem` (`self.K2_GetComponentsByClass` "/Script/Engine.StaticMeshComponent") _build_state))
  (if (> (`/Game/FirstPersonBP/Blueprints/FirstPersonCharacter.RaftPlanks` character) 0)
    (`PrimitiveComponent.SetMaterial` _output 0 (`|GetArrayItem` (`self.ComponentOrigMaterials`) _build_state))
    (`PrimitiveComponent.SetCollisionResponseToAllChannels` _output "ECR_Block")
    (`/Engine/EditorBlueprintResources/StandardMacros.IncrementInt` (`self.build state`)
      (:`  `
        (`/Engine/EditorBlueprintResources/StandardMacros.DecrementInt` (`/Game/FirstPersonBP/Blueprints/FirstPersonCharacter.RaftPlanks` character)
          (:`  `
            (if (== (`self.Build State`) (`KismetArrayLibrary.Array_Length` (`self.ComponentOrigMaterials`)))
              (set `self.is build` true))))))))

(fn `UserConstructionScript`
  (bind _returnvalue (`self.K2_GetComponentsByClass` "/Script/Engine.StaticMeshComponent"))
  (if (`self.is build`)
    (for _array_element _returnvalue
      (`PrimitiveComponent.SetCollisionResponseToAllChannels` _array_element "ECR_Block"))
    (else
      (for (_array_element_2 _array_index) _returnvalue
        (`KismetArrayLibrary.Array_Set` (`self.ComponentOrigMaterials`) _array_index (`PrimitiveComponent.GetMaterial` _array_element_2 0) true)
        (`PrimitiveComponent.SetMaterial` _array_element_2 0 "/Game/Models/raft/green.green")))))