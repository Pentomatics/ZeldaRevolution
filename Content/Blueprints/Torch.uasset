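; Torch actor that can catch fire from other burning objects and be picked up by a character.
; When its trigger starts overlapping a TorchSwitch or another Torch that is on fire, it calls Ignite, which shows the Fire component and sets OnFire.
; Activate calls PickUpTorch on a character without a torch, then destroys this actor.
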(event `/Game/Blueprints/IFlammable.Ignite`
  (`SceneComponent.SetVisibility` (`self.Fire`) true false)
  (set `self.onFire` true))

(event `self.TorchTrigger.OnComponentBeginOverlap`
  (params (OverlappedComponent :type "PrimitiveComponent Object Reference") (OtherActor :type "Actor Object Reference") (OtherComp :type "PrimitiveComponent Object Reference") (OtherBodyIndex :type Integer) (bFromSweep :type Boolean) (SweepResult :type "HitResult Structure (by ref)"))
  (bind _astorch_switch (cast `/Game/Blueprints/TorchSwitch` OtherActor)
    (:`then`
      (if (`/Game/Blueprints/TorchSwitch.onFire` _astorch_switch)
        (`/Game/Blueprints/IFlammable.Ignite` :!label _label)))
    (:`CastFailed`
      (bind _astorch (cast `/Game/Blueprints/Torch` OtherActor))
      (if (`/Game/Blueprints/Torch.onFire` _astorch)
        (goto _label)))))

(event `/Game/FirstPersonBP/ITraceable.Activate`
  (params (Character :type "/Game/FirstPersonBP/Blueprints/FirstPersonCharacter Object Reference") (Component :type "ActorComponent Object Reference"))
  (if (not (`/Game/FirstPersonBP/Blueprints/FirstPersonCharacter.hasTorch` Character))
    (`/Game/FirstPersonBP/Blueprints/FirstPersonCharacter.PickUpTorch` Character)
    (`self.K2_DestroyActor`)))

(fn `UserConstructionScript`)