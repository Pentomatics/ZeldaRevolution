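; Labyrinth is an actor that swaps background music as the first-person player enters or leaves its Box trigger.
; It mutes LabyrinthMusic on BeginPlay, then crossfades it with Music through short AdjustVolume calls on their audio components.
; Overlap events act only when the other actor's class is exactly FirstPersonCharacter, fading labyrinth music in on entry and restoring the regular track on exit.
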(event `self.ReceiveBeginPlay`
  (`AudioComponent.AdjustVolume` (`AmbientSound.AudioComponent` (`self.labyrinth music`)) 0.0 0.0))

(event `self.Box.OnComponentBeginOverlap`
  (params (OverlappedComponent :type "PrimitiveComponent Object Reference") (OtherActor :type "Actor Object Reference") (OtherComp :type "PrimitiveComponent Object Reference") (OtherBodyIndex :type Integer) (bFromSweep :type Boolean) (SweepResult :type "HitResult Structure (by ref)"))
  (if (== (`GameplayStatics.GetObjectClass` OtherActor) "/Game/FirstPersonBP/Blueprints/FirstPersonCharacter.FirstPersonCharacter_C")
    (`AudioComponent.AdjustVolume` (`AmbientSound.AudioComponent` (`self.labyrinth music`)) 0.5 0.5)
    (`AudioComponent.AdjustVolume` (`AmbientSound.AudioComponent` (`self.Music`)) 0.5 0.0)))

(event `self.Box.OnComponentEndOverlap`
  (params (OverlappedComponent :type "PrimitiveComponent Object Reference") (OtherActor :type "Actor Object Reference") (OtherComp :type "PrimitiveComponent Object Reference") (OtherBodyIndex :type Integer))
  (if (== (`GameplayStatics.GetObjectClass` OtherActor) "/Game/FirstPersonBP/Blueprints/FirstPersonCharacter.FirstPersonCharacter_C")
    (`AudioComponent.AdjustVolume` (`AmbientSound.AudioComponent` (`self.Music`)) 0.5 0.5)
    (`AudioComponent.AdjustVolume` (`AmbientSound.AudioComponent` (`self.labyrinth music`)) 0.5 0.0)))

(fn `UserConstructionScript`)