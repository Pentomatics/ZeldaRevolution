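; Eye switch for the labyrinth that opens three linked blocks when its eye is shot with an arrow.
; A DoOnce on the eye component's hit event gates a class check for Arrow, so only the first hit of any kind is evaluated.
; An arrow hit plays the item-get jingle, then unlocks Block0, Block1 and Block2 in a short staggered sequence.
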(event `self.eye_switch_eye.OnComponentHit`
  (params (HitComponent :type "PrimitiveComponent Object Reference") (OtherActor :type "Actor Object Reference") (OtherComp :type "PrimitiveComponent Object Reference") (NormalImpulse :type "Vector Structure") (Hit :type "HitResult Structure (by ref)"))
  (`/Engine/EditorBlueprintResources/StandardMacros.DoOnce` false
    (:`Completed`
      (if (== (`GameplayStatics.GetObjectClass` OtherActor) "/Game/Blueprints/Arrow.Arrow_C")
        (`GameplayStatics.PlaySound2D` "/Game/Sounds/WW_Get_Item.WW_Get_Item")
        (`/Game/Blueprints/labyrinth_block_special.UnlockDoor` (`self.block0`))
        (`KismetSystemLibrary.Delay` 0.2)
        (`/Game/Blueprints/labyrinth_block_special.UnlockDoor` (`self.block1`))
        (`KismetSystemLibrary.Delay` 0.2)
        (`/Game/Blueprints/labyrinth_block_special.UnlockDoor` (`self.block2`))))))

(fn `UserConstructionScript`)