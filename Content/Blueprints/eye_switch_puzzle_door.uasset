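; Puzzle door, named for an eye switch puzzle, that slides upward with 2D block-slide sounds once unlocked.
; UnlockDoor opens it immediately through the DoorUp timeline, while LockDoor only clears the Unlocked flag.
; While unlocked, the first-person character's overlap reopens it on entry and reverses the timeline on exit.
; An Unlockable flag skips the first unlocked overlap so the opening sound does not repeat.
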(event `LockDoor`
  (set `self.unlocked` false))

(event `self.ReceiveBeginPlay`
  ;[1 1 1] prevent opening sound from playing two times after unlock
  (set `self.unlockable` (not (`self.unlocked`))))

(event `UnlockDoor`
  (set `self.unlocked` true)
  (`GameplayStatics.PlaySound2D` "/Game/Sounds/WW_Block_Slide.WW_Block_Slide" :!label _label)
  (bind (_direction _doorup) (`Timeline|DoorUp` :!label _label_2)
    (:`Update`
      (`SceneComponent.K2_SetRelativeLocation` (`self.Door`) (`KismetMathLibrary.VLerp` (0.0 0.0 0.0) (0.0 0.0 999.0) _doorup) false false))
    (:`Finished`
      (`GameplayStatics.PlaySound2D` "/Game/Sounds/WW_Block_Slide_End.WW_Block_Slide_End"))))

(event `self.ReceiveActorBeginOverlap`
  (params (OtherActor :type "Actor Object Reference"))
  (if (== (`GameplayStatics.GetObjectClass` OtherActor) "/Game/FirstPersonBP/Blueprints/FirstPersonCharacter.FirstPersonCharacter_C")
    ;[1 1 1] prevent opening sound from playing two times after unlock
    (if (and (`self.unlockable`) (`self.unlocked`))
      (set `self.unlockable` false)
      (elif (`self.unlocked`)
        (goto _label)))))

(event `self.ReceiveActorEndOverlap`
  (params (OtherActor :type "Actor Object Reference"))
  (if (and (== (`GameplayStatics.GetObjectClass` OtherActor) "/Game/FirstPersonBP/Blueprints/FirstPersonCharacter.FirstPersonCharacter_C") (`self.unlocked`))
    (`GameplayStatics.PlaySound2D` "/Game/Sounds/WW_Block_Slide.WW_Block_Slide")
    (goto _label_2 :!via `Reverse`)))

(fn `UserConstructionScript`)