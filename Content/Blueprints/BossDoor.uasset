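; BossDoor is a lockable boss door that slides upward for the first-person character and switches the music.
; UnlockDoor sets a flag and opens it immediately; LockDoor only clears the flag.
; While unlocked, overlap begin and end play or reverse a timeline that lerps the door's height, with slide sounds.
; The first timeline update activates the entering music and mutes the level music, guarded by a DoOnce.
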(event `LockDoor`
  (set `self.unlocked` false))

(event `UnlockDoor`
  (set `self.unlocked` true)
  (`GameplayStatics.PlaySound2D` "/Game/Sounds/WW_Block_Slide.WW_Block_Slide" :!label _label)
  (bind (_direction _doorup) (`Timeline|DoorUp` :!label _label_2)
    (:`Update`
      (`SceneComponent.K2_SetRelativeLocation` (`self.Door`) (`KismetMathLibrary.VLerp` (0.0 0.0 0.0) (0.0 0.0 799.0) _doorup) false false)
      (`/Engine/EditorBlueprintResources/StandardMacros.DoOnce` false
        (:`Completed`
          (`ActorComponent.Activate` (`AmbientSound.AudioComponent` (`self.Entering Music`)) false)
          (`AudioComponent.AdjustVolume` (`AmbientSound.AudioComponent` (`self.Level Music`)) 0.0 0.0))))
    (:`Finished`
      (`GameplayStatics.PlaySound2D` "/Game/Sounds/WW_Block_Slide_End.WW_Block_Slide_End"))))

(event `self.ReceiveActorBeginOverlap`
  (params (OtherActor :type "Actor Object Reference"))
  (if (== (`GameplayStatics.GetObjectClass` OtherActor) "/Game/FirstPersonBP/Blueprints/FirstPersonCharacter.FirstPersonCharacter_C")
    (if (`self.unlocked`)
      (goto _label))))

(event `self.ReceiveActorEndOverlap`
  (params (OtherActor :type "Actor Object Reference"))
  (if (and (== (`GameplayStatics.GetObjectClass` OtherActor) "/Game/FirstPersonBP/Blueprints/FirstPersonCharacter.FirstPersonCharacter_C") (`self.unlocked`))
    (`GameplayStatics.PlaySound2D` "/Game/Sounds/WW_Block_Slide.WW_Block_Slide")
    (goto _label_2 :!via `Reverse`)))

(fn `UserConstructionScript`)