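; ShipLadder is a ladder Blueprint that marks where the first-person player can climb.
; Begin and end overlap events on its ClimbingArea component set and clear IsInClimbingArea on an overlapping FirstPersonCharacter, filtered by exact class.
; It contains no movement logic and only toggles that flag on the character.
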(event `self.ClimbingArea.OnComponentBeginOverlap`
  (params (OverlappedComponent :type "PrimitiveComponent Object Reference") (OtherActor :type "Actor Object Reference") (OtherComp :type "PrimitiveComponent Object Reference") (OtherBodyIndex :type Integer) (bFromSweep :type Boolean) (SweepResult :type "HitResult Structure (by ref)"))
  (if (== (`GameplayStatics.GetObjectClass` OtherActor) "/Game/FirstPersonBP/Blueprints/FirstPersonCharacter.FirstPersonCharacter_C")
    (bind _asfirst_person_character (cast `/Game/FirstPersonBP/Blueprints/FirstPersonCharacter` OtherActor))
    (set `/Game/FirstPersonBP/Blueprints/FirstPersonCharacter.isInClimbingArea` true _asfirst_person_character)))

(event `self.ClimbingArea.OnComponentEndOverlap`
  (params (OverlappedComponent :type "PrimitiveComponent Object Reference") (OtherActor :type "Actor Object Reference") (OtherComp :type "PrimitiveComponent Object Reference") (OtherBodyIndex :type Integer))
  (if (== (`GameplayStatics.GetObjectClass` OtherActor) "/Game/FirstPersonBP/Blueprints/FirstPersonCharacter.FirstPersonCharacter_C")
    (bind _asfirst_person_character (cast `/Game/FirstPersonBP/Blueprints/FirstPersonCharacter` OtherActor))
    (set `/Game/FirstPersonBP/Blueprints/FirstPersonCharacter.isInClimbingArea` false _asfirst_person_character)))

(fn `UserConstructionScript`)