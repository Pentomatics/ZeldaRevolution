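; TorchSwitch is a puzzle switch that catches fire when its trigger begins overlapping a burning Torch or another burning TorchSwitch.
; Ignite shows the Fire component, sets OnFire and, if the parent actor implements ISolvable, sends it OnActorActivatedMessage with itself.
; The construction script hides Fire unless OnFire is set, so a switch can start lit; nothing here extinguishes it.
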(event `/Game/Blueprints/IFlammable.Ignite`
  (bind _returnvalue (`self.GetParentActor` self))
  (`SceneComponent.SetVisibility` (`self.Fire`) true false)
  (set `self.onFire` true)
  (if (`KismetSystemLibrary.DoesImplementInterface` _returnvalue "/Game/Blueprints/ISolvable.ISolvable_C")
    (message `/Game/Blueprints/ISolvable.OnActorActivated` _returnvalue self)))

(event `self.TorchSwitchTrigger.OnComponentBeginOverlap`
  (params (OverlappedComponent :type "PrimitiveComponent Object Reference") (OtherActor :type "Actor Object Reference") (OtherComp :type "PrimitiveComponent Object Reference") (OtherBodyIndex :type Integer) (bFromSweep :type Boolean) (SweepResult :type "HitResult Structure (by ref)"))
  (bind _astorch (cast `/Game/Blueprints/Torch` OtherActor)
    (:`then`
      (if (`/Game/Blueprints/Torch.onFire` _astorch)
        (`self.Ignite` :!label _label)))
    (:`CastFailed`
      (bind _astorch_switch (cast `/Game/Blueprints/TorchSwitch` OtherActor))
      (if (`/Game/Blueprints/TorchSwitch.onFire` _astorch_switch)
        (goto _label)))))

(fn `UserConstructionScript`
  (if (not (`self.onFire`))
    (`SceneComponent.SetVisibility` (`self.Fire`) false false)))